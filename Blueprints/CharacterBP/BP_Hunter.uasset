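; BP_Hunter is the Hunter character Blueprint, handling first-person shooting, reloading and match UI.
; Fire plays an animation and calls server and, on remotes, client shoot events running a camera line trace despite "Projectile" names, with hard-coded aim correction, damage by hit bone and ammo decrement.
; Reload instantly spends a loader to refill ammo.
; Multicast-named events create and update the timer widget and show the win screen.
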(event Custom|SetIsFiring
  (params (isFiring :type Boolean))
  ;[1 0.04995 0.0595] Server Functions
  (Variables|States|SetisFiring isFiring))

(event Custom|SetIsReloading
  (params (isRelaoding :type Boolean))
  ;[1 0.04995 0.0595] Server Functions
  (Variables|States|SetisReloading isRelaoding))

(event Custom|DisplayWinInterface_Multicast
  (params (WinText :type Text))
  ;[1 0.04995 0.0595] Server Functions
  (Viewport|RemoveAllWidgets)
  (bind _returnvalue (UserInterface|CreateWidget "/Game/FirstPersonBP/UserInterface/PlayersInterface/BaseWinInterface.BaseWinInterface_C"))
  (Default|SetWinText _returnvalue WinText)
  (UserInterface|Viewport|AddtoViewport _returnvalue 0))

(event Custom|RemoveInterfaces
  ;[1 0.04995 0.0595] Server Functions
  (Viewport|RemoveAllWidgets))

(event Custom|ShootHunterProjectile_Server
  (params (Controller :type Controller%20Object%20Reference))
  ;[1 0.04995 0.0595] Server Functions
  (CallFunction|Shoot Controller))

(event Custom|ShootHunterProjectile_Client
  (params (Controller :type Controller%20Object%20Reference))
  ;[1 0.04995 0.0595] Server Functions
  (CallFunction|Shoot Controller))

(event Custom|UpdateTimeInterface_Multicast
  (params (Minutes :type Integer) (Seconds :type Integer))
  ;[1 0.04995 0.0595] Server Functions
  (CallFunction|UpdateTimeInterface Minutes Seconds))

(event Custom|CreateTimeInterface_Multicast
  ;[1 0.04995 0.0595] Server Functions
  (CallFunction|CreateTimeInterface))

(event EventBeginPlay
  (|CallParentFunction))

(event Input|ActionEvents|InputActionReload
  ;[1 1 1] InputAction Reload
  (:Pressed
    (bind _canreload (CallFunction|CanReload))
    (if _canreload
      (CallFunction|SetIsReloading true)
      (Variables|Attributes|SetLoader (- (Variables|Attributes|GetLoader) 1))
      (Variables|Default|SetAmmo (Variables|Attributes|GetAmmoInLoader))))
  (:Released
    (CallFunction|SetIsReloading false)))

(event Input|ActionEvents|InputActionFire
  (bind _returnvalue (Pawn|GetController))
  ;[1 1 1] InputAction Fire
  (:Pressed
    (bind _hasenoughammo (CallFunction|CanShoot (Variables|Default|GetAmmo)))
    (if _hasenoughammo
      (CallFunction|SetIsFiring true)
      (CallFunction|PlayShootAnimation)
      (Networking|SwitchHasAuthority
        (:Authority
          _)
        (:Remote
          (CallFunction|ShootHunterProjectileClient _returnvalue)))
      (CallFunction|ShootHunterProjectileServer _returnvalue)))
  (:Released
    (CallFunction|SetIsFiring false)))

(fn ConstructionScript
  (|CallParentFunction))

(fn Shoot
  (params (Controller :type Controller%20Object%20Reference))
  (bind _returnvalue (Pawn|GetControlRotation Controller :!class /Script/Engine.Controller))
  (bind _firstpersoncamera (Variables|Default|GetFirstPersonCamera))
  (bind _returnvalue_2 (Transformation|GetWorldLocation _firstpersoncamera))
  (bind (_pitch _yaw _roll) (Class|KismetMathLibrary|BreakRot _returnvalue))
  (bind _outhit (Collision|LineTraceForObjects _returnvalue_2 (+ _returnvalue_2 (* (Math|Vector|GetForwardVector (Class|KismetMathLibrary|MakeRot (+ _pitch -0.7) (+ _yaw 0.75) _roll)) 1e+04)) (Utilities|Array|MakeArray "ObjectTypeQuery1" "ObjectTypeQuery2") false 0 "ForDuration"))
  (CallFunction|DamageTargetbyBone (.HitActor (Collision|BreakHitResult _outhit)) (.HitBoneName (Collision|BreakHitResult _outhit)))
  (Variables|Default|SetAmmo (- (Variables|Default|GetAmmo) 1)))

(fn CreateTimeInterface
  (bind _returnvalue (UserInterface|CreateWidget "/Game/FirstPersonBP/UserInterface/PlayersInterface/TimeInterface.TimeInterface_C"))
  (bind _output_get (Variables|Default|SetTimeInterface _returnvalue))
  (UserInterface|Viewport|AddtoViewport _output_get 0))

(fn UpdateTimeInterface
  (params (Minutes :type Integer) (Seconds :type Integer))
  (Default|UpdateTime (Variables|Default|GetTimeInterface) Minutes Seconds))

(fn CanReload
  (return (Math|Boolean|ANDBoolean (> (Variables|Attributes|GetLoader) 0) (not (Variables|Default|GetIsPause)) (!= (Variables|Default|GetAmmo) (Variables|Attributes|GetAmmoInLoader)))))
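; Byormi character Blueprint that adds a networked hitscan weapon, fired with the Fire input, on top of its parent class.
; Firing checks ammo and plays the animation, then calls the server shoot event, plus the client one on remotes.
; Both events run Shoot, which line-traces from the first-person camera, applies bone-based damage and decrements ammo.
; Trace direction uses control rotation with hardcoded offsets for a centring bug, with debug drawing enabled.
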(event Custom|ByormiShoot_Server
  (params (Controller :type Controller%20Object%20Reference))
  ;[1 1 1] Server Side
  (CallFunction|Shoot Controller))

(event Custom|ByormiShoot_Client
  (params (Controller :type Controller%20Object%20Reference))
  ;[1 1 1] Server Side
  (CallFunction|Shoot Controller))

(event EventBeginPlay
  (|CallParentFunction))

(event Input|ActionEvents|InputActionFire
  (bind _returnvalue (Pawn|GetController))
  ;[1 1 1] InputAction Fire
  (:Pressed
    (bind _hasenoughammo (CallFunction|CanShoot (Variables|Default|GetAmmo)))
    (if _hasenoughammo
      (CallFunction|PlayShootAnimation)
      (Networking|SwitchHasAuthority
        (:Authority
          _)
        (:Remote
          (CallFunction|ByormiShootClient _returnvalue)))
      (CallFunction|ByormiShootServer _returnvalue))))

(fn ConstructionScript
  (|CallParentFunction))

(fn Shoot
  (params (Controller :type Controller%20Object%20Reference))
  (bind _returnvalue (Pawn|GetControlRotation Controller :!class /Script/Engine.Controller))
  (bind _firstpersoncamera (Variables|Default|GetFirstPersonCamera))
  (bind _returnvalue_2 (Transformation|GetWorldLocation _firstpersoncamera))
  (bind (_pitch _yaw _roll) (Class|KismetMathLibrary|BreakRot _returnvalue))
  (bind _outhit (Collision|LineTraceForObjects _returnvalue_2 (+ _returnvalue_2 (* (Math|Vector|GetForwardVector (Class|KismetMathLibrary|MakeRot (+ _pitch -0.7) (+ _yaw 0.75) _roll)) 1e+04)) (Utilities|Array|MakeArray "ObjectTypeQuery1" "ObjectTypeQuery2") false 0 "ForDuration"))
  (CallFunction|DamageTargetbyBone (.HitActor (Collision|BreakHitResult _outhit)) (.HitBoneName (Collision|BreakHitResult _outhit)))
  (Variables|Default|SetAmmo (- (Variables|Default|GetAmmo) 1)))
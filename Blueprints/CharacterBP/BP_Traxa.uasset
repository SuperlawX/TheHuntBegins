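; BP_Traxa is a playable character Blueprint that fires grenade projectiles from the first-person camera.
; Pressing Fire checks ammo through CanShoot and, only with authority, calls ShootTraxaGrenade with the controller and Capsule_BP.
; That event runs Shoot, which spawns the grenade at a gun offset rotated by control rotation and decrements Ammo.
; The input path has no branch for instances without authority, so those do not fire here.
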(event Custom|ShootTraxaGrenade
  (params (Controller :type Controller%20Object%20Reference) (GrenadeClass :type Actor%20Class%20Reference))
  ;[1 1 1] Server Side
  (CallFunction|Shoot Controller GrenadeClass))

(event EventBeginPlay
  (|CallParentFunction))

(event Input|ActionEvents|InputActionFire
  ;[1 1 1] InputAction Grenade
  (:Pressed
    (bind _hasenoughammo (CallFunction|CanShoot (Variables|Default|GetAmmo)))
    (if _hasenoughammo
      (if (Ability|HasAuthority)
        (CallFunction|ShootTraxaGrenade (Pawn|GetController) "/Game/FirstPersonBP/Blueprints/WeaponBP/Capsule_BP.Capsule_BP_C")))))

(fn ConstructionScript
  (|CallParentFunction))

(fn Shoot
  (params (Controller :type Controller%20Object%20Reference) (GrenadeClass :type Actor%20Class%20Reference))
  (bind _returnvalue (Pawn|GetControlRotation Controller :!class /Script/Engine.Controller))
  (Game|SpawnActorfromClass GrenadeClass (Math|Transform|MakeTransform (+ (Transformation|GetWorldLocation (Variables|Default|GetFirstPersonCamera)) (Math|Vector|RotateVector (Variables|Default|GetGunOffset) _returnvalue)) _returnvalue) false 0 0)
  (Variables|Default|SetAmmo (- (Variables|Default|GetAmmo) 1)))
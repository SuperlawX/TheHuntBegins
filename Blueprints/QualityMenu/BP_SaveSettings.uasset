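; BP_SaveSettings applies a graphics quality preset for the quality menu, chosen by its QualitySet value.
; LoadQualitySettings stores the passed GameMode, then switches over Low, Medium, High and Epic to send console-style commands for resolution, anti-aliasing, post-processing, shadows, textures and effects.
; A helper forwards each command to the GameMode, which then saves the preset with LoadSettings off.
; Resolution quality stays at full in every preset.
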(fn LoadQualitySettings
  (params (GameMode :type First%20Person%20Game%20Mode%20Object%20Reference))
  (Variables|Default|SetGamemode GameMode)
  (switch Utilities|FlowControl|Switch|SwitchonQualitySet (Variables|Default|GetQualitySet)
    (:NewEnumerator0
      ;[1 1 1] Low Settings
      (CallFunction|ExecuteCommand (Variables|ResolutionQuality|GetResolutionQuality%20100%25))
      (CallFunction|ExecuteCommand (Variables|AntiAliasing|GetAntiAliasing%200))
      (CallFunction|ExecuteCommand (Variables|PostProcessing|GetPostProcessing%200))
      (CallFunction|ExecuteCommand (Variables|Shadows|GetShadows%200))
      (CallFunction|ExecuteCommand (Variables|TextureQuality|GetTextureQuality%200))
      (CallFunction|ExecuteCommand (Variables|EffectsQuality|GetEffectsQuality%200)))
    (:NewEnumerator1
      ;[1 1 1] Medium Settings
      (CallFunction|ExecuteCommand (Variables|ResolutionQuality|GetResolutionQuality%20100%25))
      (CallFunction|ExecuteCommand (Variables|AntiAliasing|GetAntiAliasing%202))
      (CallFunction|ExecuteCommand (Variables|PostProcessing|GetPostProcessing%201))
      (CallFunction|ExecuteCommand (Variables|Shadows|GetShadows%201))
      (CallFunction|ExecuteCommand (Variables|TextureQuality|GetTextureQuality%201))
      (CallFunction|ExecuteCommand (Variables|EffectsQuality|GetEffectsQuality%201)))
    (:NewEnumerator2
      ;[1 1 1] High Settings
      (CallFunction|ExecuteCommand (Variables|ResolutionQuality|GetResolutionQuality%20100%25))
      (CallFunction|ExecuteCommand (Variables|AntiAliasing|GetAntiAliasing%204))
      (CallFunction|ExecuteCommand (Variables|PostProcessing|GetPostProcessing%202))
      (CallFunction|ExecuteCommand (Variables|Shadows|GetShadows%202))
      (CallFunction|ExecuteCommand (Variables|TextureQuality|GetTextureQuality%202))
      (CallFunction|ExecuteCommand (Variables|EffectsQuality|GetEffectsQuality%202)))
    (:NewEnumerator3
      ;[1 1 1] Epic Settings
      (CallFunction|ExecuteCommand (Variables|ResolutionQuality|GetResolutionQuality%20100%25))
      (CallFunction|ExecuteCommand (Variables|AntiAliasing|GetAntiAliasing%206))
      (CallFunction|ExecuteCommand (Variables|PostProcessing|GetPostProcessing%203))
      (CallFunction|ExecuteCommand (Variables|Shadows|GetShadows%203))
      (CallFunction|ExecuteCommand (Variables|TextureQuality|GetTextureQuality%203))
      (CallFunction|ExecuteCommand (Variables|EffectsQuality|GetEffectsQuality%203))))
  (Default|SaveSettings (Variables|Default|GetGamemode) (Variables|Default|GetQualitySet) false))

(fn ExecuteCommand
  (params (Command :type String))
  (Default|ExecuteCommand (Variables|Default|GetGamemode) Command))
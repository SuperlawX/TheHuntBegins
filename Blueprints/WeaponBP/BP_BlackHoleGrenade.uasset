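; BP_BlackHoleGrenade is a grenade weapon actor that runs a timed radial force effect, named as a black hole.
; Two seconds after BeginPlay it records its collision component's location, activates RadialForce, and plays a timeline that offsets that component vertically without sweeping.
; When the timeline finishes, it deactivates the force and destroys itself.
; The construction script runs the parent's and sets the force radius from BlastRadius.
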(event EventBeginPlay
  (bind _radialforce (Variables|Default|GetRadialForce))
  ;[1 1 1] Grenade LifeTime
  (Utilities|FlowControl|Delay 2.0)
  (Variables|Default|SetActorInitLocation (Transformation|GetWorldLocation (Variables|Default|GetCollisionComponent)))
  (Components|Activation|Activate _radialforce false)
  (bind _high (Timeline|MovingUpGrenade Play)
    (:Update
      (Transformation|SetWorldLocation (Variables|Default|GetCollisionComponent) (+ (Variables|Default|GetActorInitLocation) (Math|Vector|MakeVector 0.0 0.0 _high)) false))
    (:Finished
      (Components|Activation|Deactivate _radialforce)
      (Actor|DestroyActor))))

(fn ConstructionScript
  (|CallParentFunction)
  (Variables|/Script/Engine.RadialForceComponent|SetRadius (Variables|Default|GetRadialForce) (Variables|Default|GetBlastRadius)))
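; Base weapon Blueprint that handles hitscan firing, ammo, magazine-based reloading and bone-specific damage.
; TriggerFire rate-limits shots with a DoOnce and Delay, calling Shoot through server and client events.
; Shoot multicasts an offset camera-origin line trace that ignores non-Hunter characters, then scales random damage by hit bone.
; A separate FireProjectile function, not called here, spawns BP_Fumigene with a light toggle.
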(event Custom|DefineOwner
  (params (Owner :type BP%20Base%20Character%20Object%20Reference))
  (Variables|Default|SetOwnerActor Owner))

(event Custom|Reload
  ;[1 1 1] Reload Input
  (Utilities|FlowControl|DoOnce false :!label _label
    (:Completed
      (if (Variables|Attributes|GetcanBeReloaded)
        (if (< (Variables|Default|GetAmmoCurrent) (Variables|Attributes|GetAmmoMax))
          (if (> (Variables|Attributes|GetLoader) 0)
            (Variables|States|SetisReloading true)
            (Variables|Attributes|SetLoader (- (Variables|Attributes|GetLoader) 1))
            (Variables|Default|SetAmmoCurrent (Variables|Attributes|GetAmmoMax))
            (Variables|States|SetisReloading false)
            (goto _label Reset)))))))

(event Custom|WeaponShoot_Server
  (params (InController :type Controller%20Object%20Reference))
  ;[1 0 0.05908] Server Side
  (CallFunction|Shoot InController))

(event Custom|WeaponShoot_Client
  (params (InController :type Controller%20Object%20Reference))
  ;[1 0 0.05908] Server Side
  (CallFunction|Shoot InController))

(event Custom|LineTraceWeapon_Multicast
  (params (Start :type Vector) (End :type Vector) (ObjectTypes :type Array%20of%20EObjectTypeQuery%20Enums))
  ;[1 0 0.05908] Server Side
  (if true
    (bind _allcreatures (CallFunction|GetAllCreatures)))
  (bind _outhit (Collision|LineTraceForObjects Start End ObjectTypes false _allcreatures "ForDuration"))
  (CallFunction|DamageActorbyBone (.HitActor (Collision|BreakHitResult _outhit)) (.HitBoneName (Collision|BreakHitResult _outhit))))

(event Custom|TriggerFire
  (bind _owneractor (Variables|Default|GetOwnerActor))
  (bind _returnvalue (Pawn|GetController _owneractor))
  ;[1 1 1] Firing Input
  (Utilities|FlowControl|DoOnce false :!label _label
    (:Completed
      (if (and (not (Variables|States|GetisReloading)) (not (Variables|/Game/FirstPersonBP/Blueprints/CharacterBP/BP_BaseCharacter.BP_BaseCharacter_C|GetIsPause (Variables|Default|GetOwnerActor))))
        (bind _enoughammo (CallFunction|HasEnoughAmmo (Variables|Default|GetAmmoCurrent)))
        (if _enoughammo
          (Variables|States|SetisFiring true)
          (Default|PlayShootAnimation (Variables|Default|GetOwnerActor))
          (Networking|SwitchHasAuthority
            (:Authority
              _)
            (:Remote
              (CallFunction|WeaponShootClient _returnvalue)))
          (CallFunction|WeaponShootServer _returnvalue)
          (Utilities|FlowControl|Delay (Variables|Attributes|GetFireRate))
          (goto _label Reset))))))

(event Custom|TriggerStopFire
  ;[1 1 1] Firing Input
  (Variables|States|SetisFiring false))

(event EventBeginPlay
  ;[1 1 1] Set Ammo
  (Variables|Default|SetAmmoCurrent (Variables|Attributes|GetAmmoMax)))

(fn ConstructionScript)

(fn HasEnoughAmmo
  (params (Ammo :type Integer))
  ;[1 1 1] Has Enough Ammo
  (return (and (> Ammo 0) (not (Variables|/Game/FirstPersonBP/Blueprints/CharacterBP/BP_BaseCharacter.BP_BaseCharacter_C|GetIsPause (Variables|Default|GetOwnerActor))))))

(fn DamageActorbyBone
  (params (HitActor :type Actor%20Object%20Reference) (HitBone :type Name))
  (bind _damagemax (Variables|Attributes|GetDamageMax))
  (bind _damagemin (Variables|Attributes|GetDamageMin))
  (bind _returnvalue (Math|Random|RandomFloatinRange _damagemin _damagemax))
  ;[1 1 1] Damage Actor By Bone
  (switch name HitBone
    (:Default
      (LocalVariables|SetDamage _returnvalue))
    (:head
      (Development|PrintString "HEAD" :!label _label)
      (LocalVariables|SetDamage (* _returnvalue (Variables|DamageModifier|GetHeadDamageModifier)))
      (Game|Damage|ApplyDamage HitActor (LocalVariables|GetDamage) 0 self :!label _label_2))
    (:neck_01
      (goto _label))
    (:spine_01
      (Development|PrintString "BODY" :!label _label_3)
      (LocalVariables|SetDamage (* _returnvalue (Variables|DamageModifier|GetBodyDamageModifier)))
      (goto _label_2))
    (:spine_02
      (goto _label_3))
    (:pelvis
      (goto _label_3))
    (:upperarm_l
      (Development|PrintString "ARMS & LEGS" :!label _label_4)
      (LocalVariables|SetDamage (* _returnvalue 0.5))
      (goto _label_2))
    (:upperarm_r
      (goto _label_4))
    (:lowerarm_l
      (goto _label_4))
    (:lowerarm_r
      (goto _label_4))
    (:hand_l
      (goto _label_4))
    (:hand_r
      (goto _label_4))
    (:thigh_l
      (goto _label_4))
    (:thigh_r
      (goto _label_4))
    (:calf_l
      (goto _label_4))
    (:calf_r
      (goto _label_4))
    (:foot_l
      (Development|PrintString "FEET" :!label _label_5)
      (LocalVariables|SetDamage (* _returnvalue (Variables|DamageModifier|GetFeet&HandsDamageModifier)))
      (goto _label_2))
    (:foot_r
      (goto _label_5))
    (:ball_l
      (goto _label_5))
    (:ball_r
      (goto _label_5))))

(fn Shoot
  (params (InController :type Controller%20Object%20Reference))
  (bind _returnvalue (Pawn|GetControlRotation InController :!class /Script/Engine.Controller))
  (bind _owneractor (Variables|Default|GetOwnerActor))
  (bind (_pitch _yaw _roll) (Class|KismetMathLibrary|BreakRot _returnvalue))
  (bind _firstpersoncamera (Variables|/Game/FirstPersonBP/Blueprints/CharacterBP/BP_BaseCharacter.BP_BaseCharacter_C|GetFirstPersonCamera _owneractor))
  (bind _returnvalue_2 (Transformation|GetWorldLocation _firstpersoncamera))
  ;[1 1 1] LineTrace
  (CallFunction|LineTraceWeaponMulticast _returnvalue_2 (+ _returnvalue_2 (* (Math|Vector|GetForwardVector (Class|KismetMathLibrary|MakeRot (+ _pitch -0.7) (+ _yaw 0.75) _roll)) (Variables|Attributes|GetRange))) (Utilities|Array|MakeArray "ObjectTypeQuery1" "ObjectTypeQuery1"))
  ;[1 1 1] Remove Ammo
  (Variables|Default|SetAmmoCurrent (- (Variables|Default|GetAmmoCurrent) 1)))

(fn FireProjectile
  (bind _shootdirection (Variables|Default|GetShootDirection))
  ;[1 1 1] FireProjectile
  (Rendering|SetVisibility (Variables|Default|GetFireLight) true false)
  (Game|SpawnActorfromClass "/Game/FirstPersonBP/Blueprints/WeaponBP/BP_Fumigene.BP_Fumigene_C" (Math|Transform|MakeTransform (Transformation|GetWorldLocation _shootdirection) (Transformation|GetWorldRotation _shootdirection)) true 0 0)
  (Rendering|SetVisibility (Variables|Default|GetFireLight) false false))

(fn GetAllCreatures
  (bind _outactors (Actor|GetAllActorsOfClass "/Game/FirstPersonBP/Blueprints/CharacterBP/BP_BaseCharacter.BP_BaseCharacter_C"))
  (bind _output_get (LocalVariables|SetActors _outactors))
  (for _array_element _output_get
    (Utilities|Casting|CastToBP_Hunter _array_element)
    (Utilities|Array|RemoveItem _output_get _array_element))
  (return (LocalVariables|GetActors)))
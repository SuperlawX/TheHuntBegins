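; BP_BearTrap is a projectile-based bear trap weapon, meant to catch the Hunter stepping on it.
; Any actor overlapping its TriggerBox takes damage and switches on a RadialForce component, which deactivates after TrapDuration.
; The construction script sizes the force from ForceRadius.
; The projectile-stop event is empty, and the lifespan setter is unconnected, so it never runs.
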(event OnProjectileStop(ProjectileMovement)
  (params (ImpactResult :type Hit%20Result%20Structure%20%28by%20ref%29))
  ;[1 1 1] On Projectile Stop
)

(event OnComponentBeginOverlap(TriggerBox)
  (params (OtherActor :type Actor%20Object%20Reference) (OtherComp :type Primitive%20Component%20Object%20Reference) (OtherBodyIndex :type Integer) (bFromSweep :type Boolean) (SweepResult :type Hit%20Result%20Structure%20%28by%20ref%29))
  ;[1 1 1] The Hunter Walks on the BearTrap
  (Development|PrintString "Clap")
  (Components|Activation|Activate (Variables|Default|GetRadialForce) false)
  (Game|Damage|ApplyDamage OtherActor (Variables|Default|GetBaseDamage) 0 self)
  (Utilities|FlowControl|Delay (Variables|Default|GetTrapDuration))
  (Components|Activation|Deactivate (Variables|Default|GetRadialForce)))

(fn ConstructionScript
  (Variables|/Script/Engine.RadialForceComponent|SetRadius (Variables|Default|GetRadialForce) (Variables|Default|GetForceRadius)))
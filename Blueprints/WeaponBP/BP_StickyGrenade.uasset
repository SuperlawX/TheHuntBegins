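; BP_StickyGrenade is a projectile grenade that sticks to what it hits and explodes when its lifetime ends.
; On hit, it pushes the hit component, stops moving, attaches to the actor and disables collision.
; The timer from BeginPlay triggers radial damage, excluding actors of ignored classes, then destroys the grenade.
; Damage fires inside the actor-gathering loop, once per ignored actor found, so none occurs without one.
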(event OnComponentHit(CollisionComponent)
  (params (OtherActor :type Actor%20Object%20Reference) (OtherComp :type Primitive%20Component%20Object%20Reference) (NormalImpulse :type Vector) (Hit :type Hit%20Result%20Structure%20%28by%20ref%29))
  ;[1 1 1] Stick to mesh
  (Physics|AddImpulse OtherComp NormalImpulse "None" false)
  (Components|Movement|StopMovementImmediately (Variables|Default|GetProjectileMovement))
  (Class|Actor|AttachRootComponenttoActor OtherActor "None" "KeepWorldPosition" true)
  (Collision|SetCollisionEnabled (Variables|Default|GetCollisionComponent) "NoCollision"))

(event Custom|Explode
  (bind _ignoredclass (Variables|Default|GetIgnoredClass))
  ;[1 1 1] Explode
  (for _index (range 0 (- (Utilities|Array|Length _ignoredclass) 1))
    (bind _outactors (Actor|GetAllActorsOfClass (Utilities|Array|Get(acopy) _ignoredclass _index)))
    (for _index_2 (range 0 (- (Utilities|Array|Length _outactors) 1))
      (Utilities|Array|Add (Variables|Default|GetIgnoredActors) (Utilities|Array|Get(acopy) _outactors _index_2))
      (Game|Damage|ApplyRadialDamage (Variables|Default|GetBaseDamage) (Transformation|GetActorLocation) (Variables|Default|GetBlastRadius) 0 (Variables|Default|GetIgnoredActors) self 0 false "ECC_Visibility"))))

(event EventBeginPlay
  ;[1 1 1] Grenade LifeTime
  (Utilities|FlowControl|Delay (Variables|Default|GetLifeTime))
  (CallFunction|Explode)
  (Actor|DestroyActor))

(fn ConstructionScript
  (|CallParentFunction)
  (Components|Sphere|SetSphereRadius (Variables|Default|GetCollisionComponent) (Variables|Default|GetStickyRadius) true))
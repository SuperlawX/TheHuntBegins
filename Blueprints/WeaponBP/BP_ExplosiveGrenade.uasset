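; BP_ExplosiveGrenade is a timed explosive that deals radial damage at its location once its lifetime expires, then destroys itself.
; BeginPlay waits out LifeTime before calling Explode, which gathers all actors of each ignored class into an exclusion list.
; ApplyRadialDamage sits inside the inner gathering loop, so it fires once per actor found with a still-growing list, and never when none are found.
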(event Custom|Explode
  (bind _ignoredclass (Variables|Default|GetIgnoredClass))
  ;[1 1 1] Explode
  (for _index (range 0 (- (Utilities|Array|Length _ignoredclass) 1))
    (bind _outactors (Actor|GetAllActorsOfClass (Utilities|Array|Get(acopy) _ignoredclass _index)))
    (for _index_2 (range 0 (- (Utilities|Array|Length _outactors) 1))
      (Utilities|Array|Add (Variables|Default|GetIgnoredActors) (Utilities|Array|Get(acopy) _outactors _index_2))
      (Game|Damage|ApplyRadialDamage (Variables|Default|GetBaseDamage) (Transformation|GetActorLocation) (Variables|Default|GetBlastRadius) 0 (Variables|Default|GetIgnoredActors) self 0 false "ECC_Visibility"))))

(event EventBeginPlay
  ;[1 1 1] Grenade LifeTime
  (Utilities|FlowControl|Delay (Variables|Default|GetLifeTime))
  (CallFunction|Explode)
  (Actor|DestroyActor))

(fn ConstructionScript
  (|CallParentFunction))
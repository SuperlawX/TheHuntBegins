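; BP_Fumigene is a smoke grenade actor that emits smoke for a set lifetime, then removes itself.
; On BeginPlay it waits a short fuse delay, activates the Fumee effect, deactivates it after LifeTime, then destroys the actor shortly after.
; The construction script sizes BlastRadiusSphere from the BlastRadius variable, though the graphs shown never query that sphere.
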(event EventBeginPlay
  ;[1 1 1] Grenade lifetime
  (Utilities|FlowControl|Delay 2.0)
  (Components|Activation|Activate (Variables|Default|GetFumee) false)
  (Utilities|FlowControl|Delay (Variables|Default|GetLifeTime))
  (Components|Activation|Deactivate (Variables|Default|GetFumee))
  (Utilities|FlowControl|Delay 0.2)
  (Actor|DestroyActor))

(fn ConstructionScript
  (Components|Sphere|SetSphereRadius (Variables|Default|GetBlastRadiusSphere) (Variables|Default|GetBlastRadius) true))
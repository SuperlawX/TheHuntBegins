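; Explosive barrel actor that loses health from any damage and explodes once health reaches zero or below.
; The explosion applies radial damage around the barrel, then destroys the actor after a short delay, with no guard against retriggering meanwhile.
; The construction script sizes a sphere component to the same blast radius used for the damage.
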(event Custom|Explode
  (Game|Damage|ApplyRadialDamage (Variables|Default|GetBaseDamage) (Transformation|GetActorLocation) (Variables|Default|GetBlastRadius) 0 0 self 0 false "ECC_Visibility")
  (Utilities|FlowControl|Delay 0.2)
  (Actor|DestroyActor))

(event Game|Damage|EventAnyDamage
  (params (Damage :type Float%20%28single-precision%29) (DamageType :type Damage%20Type%20Object%20Reference) (InstigatedBy :type Controller%20Object%20Reference) (DamageCauser :type Actor%20Object%20Reference))
  (Variables|Default|SetHealth (- (Variables|Default|GetHealth) Damage))
  (if (<= (Variables|Default|GetHealth) 0.0)
    (CallFunction|Explode)))

(fn ConstructionScript
  (Components|Sphere|SetSphereRadius (Variables|Default|GetBlastRadiusSphere) (Variables|Default|GetBlastRadius) true))